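; Chicken character for the maze game that eats feed and lays eggs.
; On BeginPlay it adds a cow UI widget, removes a random GameInstance female name and separately draws its own, so duplicates remain possible.
; An overlap volume shows the nametag to the maze character.
; Another consumes chicken feed with sound and Niagara effects, updating the fed count; at three it spawns an egg and resets.
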(event `self.ReceiveBeginPlay`
  ; Sets animal's name and removes it from list for no duplicates
  (bind _returnvalue (`|CreateWidget` "/Game/ExpressFarmin_Project/GS_MazeProject/Resources/AnimalUI/WB_CowUI.WB_CowUI_C"))
  (`UserWidget.AddToViewport` _returnvalue 0)
  (bind _aswb_nametag (cast `/Game/ExpressFarmin_Project/GS_MazeProject/Resources/UI/Widgets/ActorWidgets/WB_Nametag` (`WidgetComponent.GetWidget` (`self.Widget`))))
  (set `self.As WB Nametag` _aswb_nametag)
  (bind _asbp_ef_game_instance (cast `/Game/ExpressFarmin_Project/GS_MazeProject/Resources/GameInstance/BP_EF_GameInstance` (`GameplayStatics.GetGameInstance`)))
  (bind _female_names (`/Game/ExpressFarmin_Project/GS_MazeProject/Resources/GameInstance/BP_EF_GameInstance.Female Names` _asbp_ef_game_instance))
  (bind _output (`|GetArrayItem` _female_names (`KismetMathLibrary.RandomInteger` (`KismetArrayLibrary.Array_Length` _female_names))))
  (`KismetArrayLibrary.Array_RemoveItem` _female_names _output)
  (set `self.MYName` _output))

(event `self.PlayerDetection.OnComponentBeginOverlap`
  (params (OverlappedComponent :type "PrimitiveComponent Object Reference") (OtherActor :type "Actor Object Reference") (OtherComp :type "PrimitiveComponent Object Reference") (OtherBodyIndex :type Integer) (bFromSweep :type Boolean) (SweepResult :type "HitResult Structure (by ref)"))
  ; Show animal's name
  (bind _asbp_maze_character (cast `/Game/ExpressFarmin_Project/GS_MazeProject/Resources/Blueprints/Character/BP_MazeCharacter` OtherActor))
  (set `self.As BP Maze Character` _asbp_maze_character)
  (`SceneComponent.SetVisibility` (`self.Widget`) true false)
  (`/Game/ExpressFarmin_Project/GS_MazeProject/Resources/UI/Widgets/ActorWidgets/WB_Nametag.ShowName` (`self.As WB Nametag`) (`self.MYName`)))

(event `self.PlayerDetection.OnComponentEndOverlap`
  (params (OverlappedComponent :type "PrimitiveComponent Object Reference") (OtherActor :type "Actor Object Reference") (OtherComp :type "PrimitiveComponent Object Reference") (OtherBodyIndex :type Integer))
  ; Show animal's name
  (cast `/Game/ExpressFarmin_Project/GS_MazeProject/Resources/Blueprints/Character/BP_MazeCharacter` OtherActor)
  (`SceneComponent.SetVisibility` (`self.Widget`) false false))

(event `self.HayDetection.OnComponentBeginOverlap`
  (params (OverlappedComponent :type "PrimitiveComponent Object Reference") (OtherActor :type "Actor Object Reference") (OtherComp :type "PrimitiveComponent Object Reference") (OtherBodyIndex :type Integer) (bFromSweep :type Boolean) (SweepResult :type "HitResult Structure (by ref)"))
  ; If chicken feed is detected it will be destroyed "eaten"
  (bind _asbp_chicken_feed (cast `/Game/ExpressFarmin_Project/GS_MazeProject/Resources/Blueprints/Interactables/BP_ChickenFeed` OtherActor))
  (`GameplayStatics.PlaySoundAtLocation` "/Game/ExpressFarmin_Project/GS_MazeProject/Resources/Audio/Animals/Eating/SofterCrunch.SofterCrunch" (`self.K2_GetActorLocation`) (struct) 1.0 1.0 0.0 null null null null)
  (`self.K2_DestroyActor` _asbp_chicken_feed)
  (`NiagaraFunctionLibrary.SpawnSystemAtLocation` "/Game/ExpressFarmin_Project/GS_MazeProject/Resources/FX/EM_Munchies2_System.EM_Munchies2_System" (`SceneComponent.K2_GetComponentLocation` (`self.Mouth`)))
  (bind _result (`/Engine/EditorBlueprintResources/StandardMacros.IncrementInt` (`self.FoodAmount`))
    (:`  `
      (`/Game/ExpressFarmin_Project/GS_MazeProject/Resources/UI/Widgets/ActorWidgets/WB_Nametag.Show Amount Fed` (`self.As WB Nametag`) (`KismetTextLibrary.Conv_IntToText` _result))
      (if (>= _result 3)
        (`self.LayEgg`)))))

(event `LayEgg`
  ; Animal eating functionality
  (`|SpawnActorFromClass` "/Game/ExpressFarmin_Project/GS_MazeProject/Resources/Blueprints/Interactables/BP_Egg.BP_Egg_C" (`SceneComponent.K2_GetComponentToWorld` (`self.Butt`)) "AdjustIfPossibleButAlwaysSpawn" "MultiplyWithRoot" null null)
  (`GameplayStatics.PlaySound2D` "/Game/ExpressFarmin_Project/GS_MazeProject/Resources/Audio/Animals/Eating/Pop.Pop" 1.0 1.0 0.0 null null)
  (bind _output_get (set `self.FoodAmount` 0))
  (`/Game/ExpressFarmin_Project/GS_MazeProject/Resources/UI/Widgets/ActorWidgets/WB_Nametag.Show Amount Fed` (`self.As WB Nametag`) (`KismetTextLibrary.Conv_IntToText` _output_get)))

(fn `UserConstructionScript`)