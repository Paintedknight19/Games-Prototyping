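; BP_GuiedNote is an interactable note in the maze project that opens a note screen when the player interacts with it.
; InteractObject creates a WB_Note widget, adds it to the viewport and makes its text, image and button visible.
; It then pauses the game, switches input to UI only and shows the mouse cursor, with no closing logic in this Blueprint.
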(event `self.Interact Object`
  (bind _returnvalue (`GameplayStatics.GetPlayerController` 0))
  (bind _returnvalue_2 (`|CreateWidget` "/Game/ExpressFarmin_Project/GS_MazeProject/Resources/UI/Actor_UIs/WB_Note.WB_Note_C"))
  (bind _output_get (set `self.Ref to WB2` _returnvalue_2))
  (`UserWidget.AddToViewport` _output_get 0)
  (`Widget.SetVisibility` (`/Game/ExpressFarmin_Project/GS_MazeProject/Resources/UI/Actor_UIs/WB_Note.TextBlock_1` _returnvalue_2) "Visible")
  (`Widget.SetVisibility` (`/Game/ExpressFarmin_Project/GS_MazeProject/Resources/UI/Actor_UIs/WB_Note.Image_0` _returnvalue_2) "Visible")
  (`Widget.SetVisibility` (`/Game/ExpressFarmin_Project/GS_MazeProject/Resources/UI/Actor_UIs/WB_Note.Button2` _returnvalue_2) "Visible")
  (`GameplayStatics.SetGamePaused` true)
  (`WidgetBlueprintLibrary.SetInputMode_UIOnlyEx` _returnvalue null)
  (set `PlayerController.bShowMouseCursor` true _returnvalue))

(fn `UserConstructionScript`)