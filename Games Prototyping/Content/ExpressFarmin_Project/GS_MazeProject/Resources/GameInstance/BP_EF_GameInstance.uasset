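; Game instance for the Express Farmin maze project that saves and restores player progress.
; SaveGame reuses or creates a BP_SaveGame in a single slot, writes player money and the current level name, then saves asynchronously.
; LoadGame asynchronously reads that slot, restores money, reopens the saved level and sets game-only input, or prints a message when no save exists.
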(event `SaveGame`
  (bind _returnvalue (`GameplayStatics.DoesSaveGameExist` "Save01"))
  (if _returnvalue
    (bind _returnvalue_2 (`GameplayStatics.LoadGameFromSlot` "Save01"))
    (set `self.SaveGame Ref` _returnvalue_2)
    (else
      (bind _returnvalue_3 (`GameplayStatics.CreateSaveGameObject` "/Game/ExpressFarmin_Project/GS_MazeProject/Resources/SaveGame/BP_SaveGame.BP_SaveGame_C"))
      (bind _output_get (set `self.SaveGame Ref` _returnvalue_3))))
  (bind _asbp_save_game (cast `/Game/ExpressFarmin_Project/GS_MazeProject/Resources/SaveGame/BP_SaveGame` _output_get))
  (set `/Game/ExpressFarmin_Project/GS_MazeProject/Resources/SaveGame/BP_SaveGame.Player Money` (`self.Player Money`) _asbp_save_game)
  (bind _returnvalue_4 (`GameplayStatics.GetCurrentLevelName` true))
  (set `/Game/ExpressFarmin_Project/GS_MazeProject/Resources/SaveGame/BP_SaveGame.CurrentLevel` _returnvalue_4 _asbp_save_game)
  (`AsyncActionHandleSaveGame.AsyncSaveGameToSlot` _asbp_save_game "Save01"))

(event `LoadGame`
  (bind _returnvalue (`GameplayStatics.DoesSaveGameExist` "Save01"))
  (if _returnvalue
    (bind _savegame (`AsyncActionHandleSaveGame.AsyncLoadGameFromSlot` "Save01")
      (:`then`
        (bind _asbp_save_game (cast `/Game/ExpressFarmin_Project/GS_MazeProject/Resources/SaveGame/BP_SaveGame` _savegame))
        (set `self.Player Money` (`/Game/ExpressFarmin_Project/GS_MazeProject/Resources/SaveGame/BP_SaveGame.Player Money` _asbp_save_game))
        (`GameplayStatics.OpenLevel` (`KismetStringLibrary.Conv_StringToName` (`/Game/ExpressFarmin_Project/GS_MazeProject/Resources/SaveGame/BP_SaveGame.CurrentLevel` _asbp_save_game)))
        (`WidgetBlueprintLibrary.SetInputMode_GameOnly` (`GameplayStatics.GetPlayerController` 0))))
    (else
      (`KismetSystemLibrary.PrintString` "Saved Game Does Not Exist"))))