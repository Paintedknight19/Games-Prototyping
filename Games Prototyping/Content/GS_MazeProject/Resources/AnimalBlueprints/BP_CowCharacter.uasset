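; BP_CowCharacter is a cow in the maze project that eats hay and turns it into milk or poop.
; Hay entering its detection volume is destroyed with a crunch and counted; the third feed spawns milk at the udder, the fourth spawns poop at the rear and resets the count.
; A player overlap volume toggles the cow's name tag.
; BeginPlay adds a cow UI widget to the viewport.
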(event `self.ReceiveBeginPlay`
  (bind _returnvalue (`|CreateWidget` "/Game/GS_MazeProject/Resources/AnimalUI/WB_CowUI.WB_CowUI_C"))
  (`UserWidget.AddToViewport` _returnvalue 0))

(event `self.PlayerDetection.OnComponentBeginOverlap`
  (params (OverlappedComponent :type "PrimitiveComponent Object Reference") (OtherActor :type "Actor Object Reference") (OtherComp :type "PrimitiveComponent Object Reference") (OtherBodyIndex :type Integer) (bFromSweep :type Boolean) (SweepResult :type "HitResult Structure (by ref)"))
  (cast `/Game/GS_MazeProject/Resources/Blueprints/Character/BP_MazeCharacter` OtherActor)
  (`SceneComponent.SetVisibility` (`self.NameTag Widget`) true false))

(event `self.PlayerDetection.OnComponentEndOverlap`
  (params (OverlappedComponent :type "PrimitiveComponent Object Reference") (OtherActor :type "Actor Object Reference") (OtherComp :type "PrimitiveComponent Object Reference") (OtherBodyIndex :type Integer))
  (cast `/Game/GS_MazeProject/Resources/Blueprints/Character/BP_MazeCharacter` OtherActor)
  (`SceneComponent.SetVisibility` (`self.NameTag Widget`) false false))

(event `self.HayDetection.OnComponentBeginOverlap`
  (params (OverlappedComponent :type "PrimitiveComponent Object Reference") (OtherActor :type "Actor Object Reference") (OtherComp :type "PrimitiveComponent Object Reference") (OtherBodyIndex :type Integer) (bFromSweep :type Boolean) (SweepResult :type "HitResult Structure (by ref)"))
  (bind _asbp_hay (cast `/Game/GS_MazeProject/Resources/Blueprints/Interactables/BP_Hay` OtherActor))
  (`GameplayStatics.PlaySoundAtLocation` "/Game/GS_MazeProject/Resources/Audio/Animals/LoudCrunch.LoudCrunch" (`self.K2_GetActorLocation`) (struct) 1.0 1.0 0.0 null null null null)
  (`self.K2_DestroyActor` _asbp_hay)
  (bind _result (`/Engine/EditorBlueprintResources/StandardMacros.IncrementInt` (`self.Food Amount`))
    (:`  `
      (if (== _result 3)
        (`self.Produce Milk`)
        (elif (== (`self.Food Amount`) 4)
          (`self.Overfed`)
          (set `self.Food Amount` 0))))))

(event `Produce Milk`
  (`|SpawnActorFromClass` "/Game/GS_MazeProject/Resources/Blueprints/Interactables/BP_Milk.BP_Milk_C" (`SceneComponent.K2_GetComponentToWorld` (`self.Udder Direction`)) "Undefined" "MultiplyWithRoot" null null)
  (`GameplayStatics.PlaySoundAtLocation` "/Game/GS_MazeProject/Resources/Audio/Other/Bucket.Bucket" (`SceneComponent.K2_GetComponentLocation` (`self.Udder Direction`)) (struct) 1.0 1.0 0.0 null null null null))

(event `Overfed`
  (`|SpawnActorFromClass` "/Game/GS_MazeProject/Resources/Blueprints/Interactables/BP_AnimalPoop.BP_AnimalPoop_C" (`SceneComponent.K2_GetComponentToWorld` (`self.Butt`)) "Undefined" "MultiplyWithRoot" null null)
  (`GameplayStatics.PlaySoundAtLocation` "/Game/GS_MazeProject/Resources/Audio/Animals/SmallFart.SmallFart" (`SceneComponent.K2_GetComponentLocation` (`self.Butt`)) (struct) 1.0 1.0 0.0 null null null null))

(fn `UserConstructionScript`)