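; Pig character for the maze game that eats hay and shows a nametag with a random female name from the game mode.
; Overlap spheres or volumes show the tag when the maze player is near and consume hay, updating the fed count.
; The fourth hay spawns poop with a sound and resets the count.
; A milk-spawning event, apparently left over from a cow, is never called.
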(event `self.ReceiveBeginPlay`
  (bind _aswb_nametag (cast `/Game/GS_MazeProject/Resources/UI/Widgets/ActorWidgets/WB_Nametag` (`WidgetComponent.GetWidget` (`self.NameTag Widget`))))
  (set `self.As WB Nametag` _aswb_nametag)
  (bind _asgm_maze_gamemode (cast `/Game/GS_MazeProject/Resources/Blueprints/Gamemode/GM_MazeGamemode` (`GameplayStatics.GetGameMode`)))
  (bind _femalenames (`/Game/GS_MazeProject/Resources/Blueprints/Gamemode/GM_MazeGamemode.FemaleNames` _asgm_maze_gamemode))
  (bind _output (`|GetArrayItem` _femalenames (`KismetMathLibrary.RandomInteger` (`KismetArrayLibrary.Array_Length` _femalenames))))
  (`KismetArrayLibrary.Array_RemoveItem` _femalenames _output)
  (set `self.MyName` _output))

(event `self.PlayerDetection.OnComponentBeginOverlap`
  (params (OverlappedComponent :type "PrimitiveComponent Object Reference") (OtherActor :type "Actor Object Reference") (OtherComp :type "PrimitiveComponent Object Reference") (OtherBodyIndex :type Integer) (bFromSweep :type Boolean) (SweepResult :type "HitResult Structure (by ref)"))
  ; Shows animal's name
  (bind _asbp_maze_character (cast `/Game/GS_MazeProject/Resources/Blueprints/Character/BP_MazeCharacter` OtherActor))
  (set `self.As BP Maze Character` _asbp_maze_character)
  (`SceneComponent.SetVisibility` (`self.NameTag Widget`) true false)
  (`/Game/GS_MazeProject/Resources/UI/Widgets/ActorWidgets/WB_Nametag.ShowName` (`self.As WB Nametag`) (`self.MyName`)))

(event `self.PlayerDetection.OnComponentEndOverlap`
  (params (OverlappedComponent :type "PrimitiveComponent Object Reference") (OtherActor :type "Actor Object Reference") (OtherComp :type "PrimitiveComponent Object Reference") (OtherBodyIndex :type Integer))
  ; Shows animal's name
  (cast `/Game/GS_MazeProject/Resources/Blueprints/Character/BP_MazeCharacter` OtherActor)
  (`SceneComponent.SetVisibility` (`self.NameTag Widget`) false false))

(event `Overfed`
  ; Cow has been fed to its limit (4 times) and will produce waste, resets food counter
  (`|SpawnActorFromClass` "/Game/GS_MazeProject/Resources/Blueprints/Interactables/BP_AnimalPoop.BP_AnimalPoop_C" (`SceneComponent.K2_GetComponentToWorld` (`self.Butt`)) "Undefined" "MultiplyWithRoot" null null)
  (`GameplayStatics.PlaySoundAtLocation` "/Game/GS_MazeProject/Resources/Audio/Animals/Eating/SmallFart.SmallFart" (`SceneComponent.K2_GetComponentLocation` (`self.Butt`)) (struct) 1.0 1.0 0.0 null null null null))

(event `self.HayDetection.OnComponentBeginOverlap`
  (params (OverlappedComponent :type "PrimitiveComponent Object Reference") (OtherActor :type "Actor Object Reference") (OtherComp :type "PrimitiveComponent Object Reference") (OtherBodyIndex :type Integer) (bFromSweep :type Boolean) (SweepResult :type "HitResult Structure (by ref)"))
  ; Animal eating functionality
  (bind _asbp_hay (cast `/Game/GS_MazeProject/Resources/Blueprints/Interactables/BP_Hay` OtherActor))
  (`GameplayStatics.PlaySoundAtLocation` "/Game/GS_MazeProject/Resources/Audio/Animals/Eating/LoudCrunch.LoudCrunch" (`self.K2_GetActorLocation`) (struct) 1.0 1.0 0.0 null null null null)
  (`self.K2_DestroyActor` _asbp_hay)
  (bind _result (`/Engine/EditorBlueprintResources/StandardMacros.IncrementInt` (`self.Food Amount`))
    (:`  `
      (`/Game/GS_MazeProject/Resources/UI/Widgets/ActorWidgets/WB_Nametag.Show Amount Fed` (`self.As WB Nametag`) (`KismetTextLibrary.Conv_IntToText` _result))
      (if (== _result 3)
        _
        (elif (== (`self.Food Amount`) 4)
          (`self.Overfed`)
          (bind _output_get (set `self.Food Amount` 0))
          (`/Game/GS_MazeProject/Resources/UI/Widgets/ActorWidgets/WB_Nametag.Show Amount Fed` (`self.As WB Nametag`) (`KismetTextLibrary.Conv_IntToText` _output_get)))))))

(event `Produce Milk`
  ; Produces Milk at food counter reaching 3
  (`|SpawnActorFromClass` "/Game/GS_MazeProject/Resources/Blueprints/Interactables/BP_Milk.BP_Milk_C" (`SceneComponent.K2_GetComponentToWorld` (`self.Udder Direction`)) "Undefined" "MultiplyWithRoot" null null)
  (`GameplayStatics.PlaySoundAtLocation` "/Game/GS_MazeProject/Resources/Audio/Other/SoundEffects/Actors/Bucket.Bucket" (`SceneComponent.K2_GetComponentLocation` (`self.Udder Direction`)) (struct) 1.0 1.0 0.0 null null null null))

(fn `UserConstructionScript`)