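; BP_BullCharacter is a maze-game bull that shows a nametag, eats hay and poops when overfed.
; BeginPlay creates a cow UI, then removes a random GM_MazeGamemode male name and separately picks another random one as its own.
; PlayerDetection overlaps toggle the nametag for the maze character.
; HayDetection destroys touched hay and updates the fed count; every third spawns poop at Butt with a sound and resets the count.
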(event `self.ReceiveBeginPlay`
  (bind _returnvalue (`|CreateWidget` "/Game/GS_MazeProject/Resources/AnimalUI/WB_CowUI.WB_CowUI_C"))
  (`UserWidget.AddToViewport` _returnvalue 0)
  (bind _aswb_nametag (cast `/Game/GS_MazeProject/Resources/UI/Widgets/WB_Nametag` (`WidgetComponent.GetWidget` (`self.NameTag Widget`))))
  (set `self.As WB Nametag` _aswb_nametag)
  (bind _asgm_maze_gamemode (cast `/Game/GS_MazeProject/Resources/Blueprints/Gamemode/GM_MazeGamemode` (`GameplayStatics.GetGameMode`)))
  (bind _malenames (`/Game/GS_MazeProject/Resources/Blueprints/Gamemode/GM_MazeGamemode.MaleNames` _asgm_maze_gamemode))
  (bind _output (`|GetArrayItem` _malenames (`KismetMathLibrary.RandomInteger` (`KismetArrayLibrary.Array_Length` _malenames))))
  (`KismetArrayLibrary.Array_RemoveItem` _malenames _output)
  (set `self.MyName` _output))

(event `self.PlayerDetection.OnComponentBeginOverlap`
  (params (OverlappedComponent :type "PrimitiveComponent Object Reference") (OtherActor :type "Actor Object Reference") (OtherComp :type "PrimitiveComponent Object Reference") (OtherBodyIndex :type Integer) (bFromSweep :type Boolean) (SweepResult :type "HitResult Structure (by ref)"))
  (bind _asbp_maze_character (cast `/Game/GS_MazeProject/Resources/Blueprints/Character/BP_MazeCharacter` OtherActor))
  (set `self.As BP Maze Character` _asbp_maze_character)
  (`SceneComponent.SetVisibility` (`self.NameTag Widget`) true false)
  (`/Game/GS_MazeProject/Resources/UI/Widgets/WB_Nametag.ShowName` (`self.As WB Nametag`) (`self.MyName`)))

(event `self.PlayerDetection.OnComponentEndOverlap`
  (params (OverlappedComponent :type "PrimitiveComponent Object Reference") (OtherActor :type "Actor Object Reference") (OtherComp :type "PrimitiveComponent Object Reference") (OtherBodyIndex :type Integer))
  (cast `/Game/GS_MazeProject/Resources/Blueprints/Character/BP_MazeCharacter` OtherActor)
  (`SceneComponent.SetVisibility` (`self.NameTag Widget`) false false))

(event `self.HayDetection.OnComponentBeginOverlap`
  (params (OverlappedComponent :type "PrimitiveComponent Object Reference") (OtherActor :type "Actor Object Reference") (OtherComp :type "PrimitiveComponent Object Reference") (OtherBodyIndex :type Integer) (bFromSweep :type Boolean) (SweepResult :type "HitResult Structure (by ref)"))
  (bind _asbp_hay (cast `/Game/GS_MazeProject/Resources/Blueprints/Interactables/BP_Hay` OtherActor))
  (`GameplayStatics.PlaySoundAtLocation` "/Game/GS_MazeProject/Resources/Audio/Animals/Eating/LoudCrunch.LoudCrunch" (`self.K2_GetActorLocation`) (struct) 1.0 1.0 0.0 null null null null)
  (`self.K2_DestroyActor` _asbp_hay)
  (bind _result (`/Engine/EditorBlueprintResources/StandardMacros.IncrementInt` (`self.Food Amount`))
    (:`  `
      (`/Game/GS_MazeProject/Resources/UI/Widgets/WB_Nametag.Show Amount Fed` (`self.As WB Nametag`) (`KismetTextLibrary.Conv_IntToText` _result))
      (if (== _result 3)
        (`self.Overfed`)
        (bind _output_get (set `self.Food Amount` 0))
        (`/Game/GS_MazeProject/Resources/UI/Widgets/WB_Nametag.Show Amount Fed` (`self.As WB Nametag`) (`KismetTextLibrary.Conv_IntToText` _output_get))))))

(event `Overfed`
  (`|SpawnActorFromClass` "/Game/GS_MazeProject/Resources/Blueprints/Interactables/BP_AnimalPoop.BP_AnimalPoop_C" (`SceneComponent.K2_GetComponentToWorld` (`self.Butt`)) "Undefined" "MultiplyWithRoot" null null)
  (`GameplayStatics.PlaySoundAtLocation` "/Game/GS_MazeProject/Resources/Audio/Animals/Eating/SmallFart.SmallFart" (`SceneComponent.K2_GetComponentLocation` (`self.Butt`)) (struct) 1.0 1.0 0.0 null null null null))

(fn `UserConstructionScript`)