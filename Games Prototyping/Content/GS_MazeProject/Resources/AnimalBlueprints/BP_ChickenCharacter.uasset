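; BP_ChickenCharacter is a maze-game chicken that eats feed and lays eggs.
; Feed entering HayDetection is destroyed after a short delay and increments FoodAmount; at the threshold, LayEgg spawns a BP_Egg at the Butt component and resets the count.
; PlayerDetection shows the ChickenScreen of a new WB_CowUI while the maze character overlaps and removes that widget on exit.
; BeginPlay also adds a separate, unstored WB_CowUI to the viewport.
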(event `self.ReceiveBeginPlay`
  (bind _returnvalue (`|CreateWidget` "/Game/GS_MazeProject/Resources/AnimalUI/WB_CowUI.WB_CowUI_C"))
  (`UserWidget.AddToViewport` _returnvalue 0))

(event `self.PlayerDetection.OnComponentBeginOverlap`
  (params (OverlappedComponent :type "PrimitiveComponent Object Reference") (OtherActor :type "Actor Object Reference") (OtherComp :type "PrimitiveComponent Object Reference") (OtherBodyIndex :type Integer) (bFromSweep :type Boolean) (SweepResult :type "HitResult Structure (by ref)"))
  (cast `/Game/GS_MazeProject/Resources/Blueprints/Character/BP_MazeCharacter` OtherActor)
  (`KismetSystemLibrary.PrintString` "Enter")
  (bind _returnvalue (`|CreateWidget` "/Game/GS_MazeProject/Resources/AnimalUI/WB_CowUI.WB_CowUI_C"))
  (bind _output_get (set `self.Reference to CowUI` _returnvalue))
  (`Widget.SetVisibility` (`/Game/GS_MazeProject/Resources/AnimalUI/WB_CowUI.ChickenScreen` _output_get) "Visible")
  (`UserWidget.AddToViewport` _returnvalue 0))

(event `self.PlayerDetection.OnComponentEndOverlap`
  (params (OverlappedComponent :type "PrimitiveComponent Object Reference") (OtherActor :type "Actor Object Reference") (OtherComp :type "PrimitiveComponent Object Reference") (OtherBodyIndex :type Integer))
  (cast `/Game/GS_MazeProject/Resources/Blueprints/Character/BP_MazeCharacter` OtherActor)
  (`KismetSystemLibrary.PrintString` "Exit")
  (`Widget.RemoveFromParent` (`self.Reference to CowUI`)))

(event `self.HayDetection.OnComponentBeginOverlap`
  (params (OverlappedComponent :type "PrimitiveComponent Object Reference") (OtherActor :type "Actor Object Reference") (OtherComp :type "PrimitiveComponent Object Reference") (OtherBodyIndex :type Integer) (bFromSweep :type Boolean) (SweepResult :type "HitResult Structure (by ref)"))
  ; If chicken feed is detected it will be destroyed "eaten"
  (bind _asbp_chicken_feed (cast `/Game/GS_MazeProject/Resources/Blueprints/Interactables/BP_ChickenFeed` OtherActor))
  (`KismetSystemLibrary.Delay` 0.5)
  (`self.K2_DestroyActor` _asbp_chicken_feed)
  (bind _result (`/Engine/EditorBlueprintResources/StandardMacros.IncrementInt` (`self.FoodAmount`))
    (:`  `
      (if (>= _result 3)
        (`self.LayEgg`)))))

(event `LayEgg`
  (`|SpawnActorFromClass` "/Game/GS_MazeProject/Resources/Blueprints/Interactables/BP_Egg.BP_Egg_C" (`SceneComponent.K2_GetComponentToWorld` (`self.Butt`)) "AdjustIfPossibleButAlwaysSpawn" "MultiplyWithRoot" null null)
  (set `self.FoodAmount` 0))

(fn `UserConstructionScript`)