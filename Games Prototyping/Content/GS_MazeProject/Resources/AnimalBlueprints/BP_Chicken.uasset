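; BP_Chicken is a maze-game chicken Blueprint that shows a nametag UI while the maze character is nearby.
; When BP_MazeCharacter enters its Box trigger, it creates a new WB_ChickenUI, makes it and its ChickenNametag visible, and adds it to the viewport.
; When the character leaves, the stored widget is removed from its parent, with debug prints on both enter and exit.
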(event `self.Box.OnComponentBeginOverlap`
  (params (OverlappedComponent :type "PrimitiveComponent Object Reference") (OtherActor :type "Actor Object Reference") (OtherComp :type "PrimitiveComponent Object Reference") (OtherBodyIndex :type Integer) (bFromSweep :type Boolean) (SweepResult :type "HitResult Structure (by ref)"))
  (cast `/Game/GS_MazeProject/Resources/Blueprints/Character/BP_MazeCharacter` OtherActor)
  (`KismetSystemLibrary.PrintString` "Enter")
  (bind _returnvalue (`|CreateWidget` "/Game/GS_MazeProject/Resources/AnimalUI/WB_ChickenUI.WB_ChickenUI_C"))
  (bind _output_get (set `self.Reference to Chicken UI` _returnvalue))
  (`Widget.SetVisibility` _output_get "Visible")
  (`Widget.SetVisibility` (`/Game/GS_MazeProject/Resources/AnimalUI/WB_ChickenUI.ChickenNametag` _output_get) "Visible")
  (`UserWidget.AddToViewport` _returnvalue 0))

(event `self.Box.OnComponentEndOverlap`
  (params (OverlappedComponent :type "PrimitiveComponent Object Reference") (OtherActor :type "Actor Object Reference") (OtherComp :type "PrimitiveComponent Object Reference") (OtherBodyIndex :type Integer))
  (cast `/Game/GS_MazeProject/Resources/Blueprints/Character/BP_MazeCharacter` OtherActor)
  (`KismetSystemLibrary.PrintString` "Exit")
  (`Widget.RemoveFromParent` (`self.Reference to Chicken UI`)))

(fn `UserConstructionScript`)