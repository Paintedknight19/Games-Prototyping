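; BP_Well is a maze interactable that turns an empty water bucket into a filled one.
; A player detection volume shows a widget while the maze character overlaps it and hides it on exit.
; When an empty bucket enters the bucket detection volume, the well spawns a water bucket at its Arrow, plays a splash sound at world origin and destroys the empty one.
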(event `self.Player Detection.OnComponentBeginOverlap`
  (params (OverlappedComponent :type "PrimitiveComponent Object Reference") (OtherActor :type "Actor Object Reference") (OtherComp :type "PrimitiveComponent Object Reference") (OtherBodyIndex :type Integer) (bFromSweep :type Boolean) (SweepResult :type "HitResult Structure (by ref)"))
  (cast `/Game/GS_MazeProject/Resources/Blueprints/Character/BP_MazeCharacter` OtherActor)
  (`SceneComponent.SetVisibility` (`self.Widget`) true false))

(event `self.Player Detection.OnComponentEndOverlap`
  (params (OverlappedComponent :type "PrimitiveComponent Object Reference") (OtherActor :type "Actor Object Reference") (OtherComp :type "PrimitiveComponent Object Reference") (OtherBodyIndex :type Integer))
  (cast `/Game/GS_MazeProject/Resources/Blueprints/Character/BP_MazeCharacter` OtherActor)
  (`SceneComponent.SetVisibility` (`self.Widget`) false false))

(event `self.Bucket Detection.OnComponentBeginOverlap`
  (params (OverlappedComponent :type "PrimitiveComponent Object Reference") (OtherActor :type "Actor Object Reference") (OtherComp :type "PrimitiveComponent Object Reference") (OtherBodyIndex :type Integer) (bFromSweep :type Boolean) (SweepResult :type "HitResult Structure (by ref)"))
  (bind _asbp_empty_water (cast `/Game/GS_MazeProject/Resources/Blueprints/Interactables/BP_EMPTY_Water` OtherActor))
  (`|SpawnActorFromClass` "/Game/GS_MazeProject/Resources/Blueprints/Interactables/BP_WATER_Bucket.BP_WATER_Bucket_C" (`SceneComponent.K2_GetComponentToWorld` (`self.Arrow`)) "Undefined" "MultiplyWithRoot" null null)
  (`GameplayStatics.PlaySoundAtLocation` "/Game/GS_MazeProject/Resources/Audio/Other/SoundEffects/WaterSplash.WaterSplash" (0.0 0.0 0.0) (struct) 1.0 1.0 0.0 null null null null)
  (`self.K2_DestroyActor` _asbp_empty_water))

(fn `UserConstructionScript`)