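; BP_Laptop is an interactable laptop actor that opens a full laptop UI for the player.
; Its PlayerDetection overlap shows a "press E to interact" widget for BP_MazeCharacter and removes it when the overlap ends.
; InteractObject creates WB_Laptop with a BPDeliveryPoint reference, shows its main screen, and switches to UI-only input with a visible cursor.
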(event `/Game/GS_MazeProject/Resources/Blueprints/BPI_InteractObject.Interact Object`
  (bind _returnvalue (`GameplayStatics.GetPlayerController` 0))
  (bind _returnvalue_2 (`|CreateWidget` "/Game/GS_MazeProject/Resources/UI/WB_Laptop.WB_Laptop_C" null (`self.As BP Delivery Point`)))
  (bind _output_get (set `self.Ref to Laptop WB` _returnvalue_2))
  (`UserWidget.AddToViewport` _output_get 0)
  (`Widget.SetVisibility` (`/Game/GS_MazeProject/Resources/UI/WB_Laptop.MainScreen` _returnvalue_2) "Visible")
  (`WidgetBlueprintLibrary.SetInputMode_UIOnlyEx` _returnvalue null)
  (set `PlayerController.bShowMouseCursor` true _returnvalue))

(event `self.Player Detection.OnComponentBeginOverlap`
  (params (OverlappedComponent :type "PrimitiveComponent Object Reference") (OtherActor :type "Actor Object Reference") (OtherComp :type "PrimitiveComponent Object Reference") (OtherBodyIndex :type Integer) (bFromSweep :type Boolean) (SweepResult :type "HitResult Structure (by ref)"))
  (cast `/Game/GS_MazeProject/Resources/Blueprints/Character/BP_MazeCharacter` OtherActor)
  (bind _returnvalue (`|CreateWidget` "/Game/GS_MazeProject/Resources/UI/Actor_UIs/WB_EtoInteract.WB_EtoInteract_C"))
  (bind _output_get (set `self.Reference to E` _returnvalue))
  (`Widget.SetVisibility` (`/Game/GS_MazeProject/Resources/UI/Actor_UIs/WB_EtoInteract.EtoInteractTextbox` _output_get) "Visible")
  (`UserWidget.AddToViewport` _returnvalue 0))

(event `self.Player Detection.OnComponentEndOverlap`
  (params (OverlappedComponent :type "PrimitiveComponent Object Reference") (OtherActor :type "Actor Object Reference") (OtherComp :type "PrimitiveComponent Object Reference") (OtherBodyIndex :type Integer))
  (cast `/Game/GS_MazeProject/Resources/Blueprints/Character/BP_MazeCharacter` OtherActor)
  (`Widget.SetVisibility` (`self.Reference to E`) "Collapsed")
  (`Widget.RemoveFromParent` (`self.Reference to E`)))

(fn `UserConstructionScript`)