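; BP_ShippingPoint is a selling point that turns ingredient actors entering its ItemDetection volume into player money.
; Overlapping actors with an AC_IngredientType component add their amount to a running per-name tally in the Ingridients map.
; It then passes the IngridientPrices lookup plus the item's AC_MonetaryValue price to MoneyUpdates on player 0's BP_MazeCharacter, plays a sale sound and destroys the item.
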(event `self.Item Detection.OnComponentBeginOverlap`
  (params (OverlappedComponent :type "PrimitiveComponent Object Reference") (OtherActor :type "Actor Object Reference") (OtherComp :type "PrimitiveComponent Object Reference") (OtherBodyIndex :type Integer) (bFromSweep :type Boolean) (SweepResult :type "HitResult Structure (by ref)"))
  (bind _returnvalue (`self.GetComponentByClass` OtherActor "/Game/GS_MazeProject/Resources/Blueprints/Interactables/AC_IngredientType.AC_IngredientType_C"))
  (bind _returnvalue_2 (`self.GetComponentByClass` OtherActor "/Game/GS_MazeProject/Resources/Blueprints/Interactables/AC_MonetaryValue.AC_MonetaryValue_C"))
  (bind _ingridients (`self.Ingridients`))
  (bind _ingredientname (`/Game/GS_MazeProject/Resources/Blueprints/Interactables/AC_IngredientType.IngredientName` _returnvalue))
  (`/Engine/EditorBlueprintResources/StandardMacros.IsValid` _returnvalue
    (:`Is Valid`
      (`BlueprintMapLibrary.Map_Add` _ingridients _ingredientname (+ (`BlueprintMapLibrary.Map_Find` _ingridients _ingredientname) (`/Game/GS_MazeProject/Resources/Blueprints/Interactables/AC_IngredientType.IngredientAmount` _returnvalue)))
      (bind _asbp_maze_character (cast `/Game/GS_MazeProject/Resources/Blueprints/Character/BP_MazeCharacter` (`GameplayStatics.GetPlayerCharacter` 0)))
      (`/Game/GS_MazeProject/Resources/Blueprints/Character/BP_MazeCharacter.Money Updates` _asbp_maze_character (+ (`BlueprintMapLibrary.Map_Find` (`self.Ingridient Prices`) (`/Game/GS_MazeProject/Resources/Blueprints/Interactables/AC_MonetaryValue.Name` _returnvalue_2)) (`/Game/GS_MazeProject/Resources/Blueprints/Interactables/AC_MonetaryValue.Price` _returnvalue_2)))
      (`GameplayStatics.PlaySound2D` "/Game/GS_MazeProject/Resources/Audio/Character/PlayerSells.PlayerSells" 1.0 1.0 0.0 null null)
      (`self.K2_DestroyActor` OtherActor))))

(fn `UserConstructionScript`)