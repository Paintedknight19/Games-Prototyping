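; BP_DeliveryPoint is a delivery spot actor that spawns purchasable farm products into the level.
; Its SpawnChickenFeed event switches on the ProductsYouCanBuy value to spawn Chicken Feed, Hay or Milk actors at the Arrow component's world transform, ignoring collisions.
; A chicken character spawn node is left unconnected and never runs.
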(event `/Game/GS_MazeProject/Resources/Blueprints/BPI_LaptopUse.SpawnChickenFeed`
  (params (`Products you can buy` :type "/Game/GS_MazeProject/Resources/Blueprints/E_ProductsToBuy Enum" :default "NewEnumerator0"))
  (switch `/Game/GS_MazeProject/Resources/Blueprints/E_ProductsToBuy` `Products you can buy`
    (:`NewEnumerator0`
      (`|SpawnActorFromClass` "/Game/GS_MazeProject/Resources/Blueprints/Interactables/BP_ChickenFeed.BP_ChickenFeed_C" (`SceneComponent.K2_GetComponentToWorld` (`self.Arrow`)) "AlwaysSpawn" "MultiplyWithRoot" null null))
    (:`NewEnumerator1`
      (`|SpawnActorFromClass` "/Game/GS_MazeProject/Resources/Blueprints/Interactables/BP_Hay.BP_Hay_C" (`SceneComponent.K2_GetComponentToWorld` (`self.Arrow`)) "AlwaysSpawn" "MultiplyWithRoot" null null))
    (:`NewEnumerator2`
      (`|SpawnActorFromClass` "/Game/GS_MazeProject/Resources/Blueprints/Interactables/BP_Milk.BP_Milk_C" (`SceneComponent.K2_GetComponentToWorld` (`self.Arrow`)) "AlwaysSpawn" "MultiplyWithRoot" null null))))

(fn `Spawn Chicken Feed`)

(fn `UserConstructionScript`)